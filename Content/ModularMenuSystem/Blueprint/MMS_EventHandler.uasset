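; Event handler for the Modular Menu System, receiving callbacks from buttons, checkboxes, comboboxes, sliders, text inputs and scrollboxes.
; Each public callback only prints debug text describing the widget event.
; PrivateButtonCallback wraps ButtonCallback: when a DialogMenu is registered, it matches common dialog button ID suffixes to remove and clear that dialog.
; Button events are forwarded to ButtonCallback whether or not a dialog closes.
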(fn ConstructionScript)

(fn ButtonCallback
  (params (ID :type Name) (Caption :type Text))
  (Development|PrintString (Utilities|String|ToString(Text) Caption)))

(fn CheckboxCallback
  (params (ID :type Name) (Caption :type Text) (Checked :type Boolean))
  (Development|PrintString (Utilities|String|Append "Checkbox " (Utilities|String|ToString(Text) Caption) ": " (Utilities|String|ToString(Boolean) Checked))))

(fn ComboboxCallback
  (params (ID :type Name) (Caption :type Text) (Selection :type String))
  (Development|PrintString (Utilities|String|Append "Combo " (Utilities|String|ToString(Text) Caption) " Selection: " Selection)))

(fn SliderCallback
  (params (ID :type Name) (Caption :type Text) (Value :type Float%20%28single-precision%29))
  (Development|PrintString (Utilities|String|Append "Slider " (Utilities|String|ToString(Text) Caption) " Value: " (Utilities|String|ToString(Float) Value))))

(fn TextInputCallback
  (params (ID :type Name) (Caption :type Text) (Text :type Text))
  (Development|PrintString (Utilities|String|Append "Text Input \"" (Utilities|String|ToString(Text) Caption) "\" changed: " (Utilities|String|ToString(Text) Text))))

(fn PrivateButtonCallback
  (params (ID :type Name) (Caption :type Text))
  (LocalVariables|SetEvtID ID)
  (LocalVariables|SetEvtCaption Caption)
  ;[1 1 1] Check whether we are registered to a dialog menu, exit if not.
  (if (not (Utilities|IsValid (Variables|MMS|GetDialogMenu)))
    (MMSCallbacks|ButtonCallback (LocalVariables|GetEvtID) (LocalVariables|GetEvtCaption))
    (else
      ;[1 1 1] Then check for common dialog button IDs.
      (if (and (Math|Boolean|ORBoolean (Utilities|String|EndsWith (Utilities|String|ToString(Name) (LocalVariables|GetEvtID)) "_DialogClose" "CaseSensitive") (Utilities|String|EndsWith (Utilities|String|ToString(Name) (LocalVariables|GetEvtID)) "_DialogYes" "CaseSensitive") (Utilities|String|EndsWith (Utilities|String|ToString(Name) (LocalVariables|GetEvtID)) "_DialogNo" "CaseSensitive") (Utilities|String|EndsWith (Utilities|String|ToString(Name) (LocalVariables|GetEvtID)) "_DialogLoad" "CaseSensitive") (Utilities|String|EndsWith (Utilities|String|ToString(Name) (LocalVariables|GetEvtID)) "_DialogSave" "CaseSensitive") (Utilities|String|EndsWith (Utilities|String|ToString(Name) (LocalVariables|GetEvtID)) "_DialogGraphicsSaveBtn" "CaseSensitive") (Utilities|String|EndsWith (Utilities|String|ToString(Name) (LocalVariables|GetEvtID)) "_DialogGraphicsCancelBtn" "CaseSensitive")) (Utilities|IsValid (Variables|MMS|GetDialogMenu)))
        ;[1 1 1] Close dialog window.
        (Default|GetMenuWidget (Variables|MMS|GetDialogMenu))
        (Widget|RemovefromParent (Variables|MMS|GetDialogMenu))
        (Variables|MMS|SetDialogMenu 0))
      (MMSCallbacks|ButtonCallback (LocalVariables|GetEvtID) (LocalVariables|GetEvtCaption)))))

(fn ScrollboxCallback
  (params (ID :type Name) (Selection :type Text) (Selected :type Boolean))
  (Development|PrintString (Utilities|String|Append "ScrollBox \"" (Utilities|String|ToString(Name) ID) "\" Selection changed: " (Utilities|String|ToString(Text) Selection))))